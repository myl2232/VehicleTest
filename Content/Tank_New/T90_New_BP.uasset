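; T90_New_BP is a player-drivable T-90 tank pawn with two tracks and two switchable cameras.
; A MovementComponent, initialized with both track components, takes per-side brake inputs, a steering vector from the forward/right axes and a signed squared-magnitude throttle.
; Each track builds itself from its instanced mesh component in both the construction script and BeginPlay.
; The SwitchCamera action toggles which of the two cameras is active.
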(event `self.ReceiveBeginPlay`
  (`|ExecutionSequence`
    (:`then_0`
      (`TankMovementComponent.Init` (`self.MovementComponent`) (`self.TrackLeft`) (`self.TrackRight`)))
    (:`then_1`
      (`TrackComponent.BuildTrack` (`self.TrackLeft`) (`self.InstanceMeshLeft`))
      (`TrackComponent.BuildTrack` (`self.TrackRight`) (`self.InstanceMeshRight`)))))

(event `InputAxis|Left Brake`
  (params (AxisValue :type "Float (single-precision)"))
  (`TankMovementComponent.SetLeftBrakeInput` (`self.MovementComponent`) AxisValue))

(event `InputAxis|MoveForward`
  (params (AxisValue :type "Float (single-precision)"))
  (bind _returnvalue (`self.GetInputAxisValue`))
  (`WheeledVehicleMovementComponent.SetThrottleInput` (`self.MovementComponent`) (* (select `bool` (< _returnvalue 0.0) :`false` 1.0 :`true` -1.0 :!type "Float (single-precision)") (+ (`KismetMathLibrary.Square` _returnvalue) (`KismetMathLibrary.Square` (`self.GetInputAxisValue`))))))

(event `InputAxis|Right Brake`
  (params (AxisValue :type "Float (single-precision)"))
  (`TankMovementComponent.SetRightBrakeInput` (`self.MovementComponent`) AxisValue))

(event `InputAxis|MoveRight`
  (params (AxisValue :type "Float (single-precision)"))
  (`TankMovementComponent.SetSteeringDirection` (`self.MovementComponent`) (`KismetMathLibrary.MakeVector2D` (`self.GetInputAxisValue`) (`self.GetInputAxisValue`))))

(event `InputAction|SwitchCamera`
  (params (Key :type "Key Structure"))
  (bind _camera2 (`self.Camera2`))
  (bind _camera (`self.Camera`))
  (:`Pressed`
    (if (`ActorComponent.IsActive` (`self.Camera`))
      (`ActorComponent.SetActive` _camera2 true false)
      (`ActorComponent.SetActive` _camera false false)
      (else
        (`ActorComponent.SetActive` _camera true false)
        (`ActorComponent.SetActive` _camera2 false false)))))

(fn `UserConstructionScript`
  (`TrackComponent.BuildTrack` (`self.TrackLeft`) (`self.InstanceMeshLeft`))
  (`TrackComponent.BuildTrack` (`self.TrackRight`) (`self.InstanceMeshRight`)))